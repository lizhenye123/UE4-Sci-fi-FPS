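; Behavior tree service that picks a Conquest capture flag as an AI pawn's objective when the service activates.
; It reads the capture points from the Conquest game state and filters them by objective state against the pawn's team, apparently skipping flags its team holds.
; Despite its name, FindClosestFlag returns the first candidate within 1000 units, otherwise a random one, and the result goes into the objective Blackboard key.
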(event `self.ReceiveActivationAI`
  (params (OwnerController :type "AIController Object Reference") (ControlledPawn :type "Pawn Object Reference"))
  ;[1 1 1] 设置交互物（旗帜）
  (bind _asbp_conquest_gs (cast `/Game/FPS/Blueprints/GameModes/Conquest/BP_Conquest_GS` (`GameplayStatics.GetGameState`)))
  (bind _pointstocapturearray (`/Game/FPS/Blueprints/GameModes/Conquest/BP_Conquest_GS.PointsToCaptureArray` _asbp_conquest_gs))
  (if (`KismetArrayLibrary.Array_IsValidIndex` _pointstocapturearray)
    (bind _flag (`self.FindClosestFlag` _pointstocapturearray ControlledPawn))
    (`/Engine/EditorBlueprintResources/StandardMacros.IsValid` _flag
      (:`Is Valid`
        (`BTFunctionLibrary.SetBlackboardValueAsObject` (`self.Objectivekey`) _flag)))))

(fn `FindClosestFlag`
  (params (CapturePoints :type "Array of /Game/FPS/Blueprints/GameObjectives/ConquestZones/BP_ConquestCapturePoint Object Reference") (SelfPawn :type "Pawn Object Reference"))
  (returns (Flag :type "/Game/FPS/Blueprints/GameObjectives/ConquestZones/BP_ConquestCapturePoint Object Reference"))
  (locals (MinDistance :type "Float (double-precision)" :default 2500000.0) (Pawn :type "Pawn Object Reference"))
  (bind _posibleflagstocapture (`self.PosibleFlagsToCapture`))
  (bind _objetivestate (`/Game/FPS/Blueprints/GameObjectives/ConquestZones/BP_ConquestCapturePoint.ObjetiveState` (`self.PossibleFlag`)))
  (`/Engine/EditorBlueprintResources/StandardMacros.IsValid` SelfPawn
    (:`Is Valid`
      (`KismetArrayLibrary.Array_Clear` (`self.PosibleFlagsToCapture`))
      (set `local.MinDistance` 250000.0)
      (set `local.Pawn` SelfPawn)
      (for _array_element CapturePoints
        (set `self.PossibleFlag` _array_element)
        (if (`|EnumEquality` _objetivestate "NewEnumerator2")
          (`KismetArrayLibrary.Array_Add` (`self.PosibleFlagsToCapture`) (`self.PossibleFlag`) :!label _label)
          (if (< (`Actor.GetDistanceTo` (`local.Pawn`) (`self.PossibleFlag`)) 1000.0)
            (return (`self.PossibleFlag`)))
          (elif (== (`/Game/FPS/Blueprints/FunctionLibrary/BP_FunctionLibrary.GetPlayerTeamFromPlayerState` (`Pawn.PlayerState` (`local.Pawn`))) 0)
            (if (`|EnumInequality` _objetivestate "NewEnumerator0")
              (goto _label))
            (elif (`|EnumInequality` _objetivestate "NewEnumerator1")
              (goto _label)))))
      (if (!= (`KismetArrayLibrary.Array_Length` (`self.PosibleFlagsToCapture`)) 0)
        (return (`|GetArrayItem` _posibleflagstocapture (`KismetMathLibrary.RandomIntegerInRange` 0 (`KismetArrayLibrary.Array_LastIndex` _posibleflagstocapture))))
        (else
          (return null))))))