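; Behavior tree service for Capture the Flag bots that writes the next move location to a blackboard vector key.
; Each tick it reads the pawn's team and checks both flags in BP_CaptureTheFlag_GS.
; A taken own flag takes priority, yet targets a point near the opposing flag.
; Otherwise the carrier heads to its own flag's base, teammates roam around the carrier, or bots go for the untaken enemy flag.
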(event `self.ReceiveTickAI`
  (params (OwnerController :type "AIController Object Reference") (ControlledPawn :type "Pawn Object Reference") (DeltaSeconds :type "Float (single-precision)"))
  (bind _team (message `/Game/FPS/Blueprints/Interfaces/iPlayerState.GetTeam` (`Pawn.PlayerState` ControlledPawn)))
  (`self.SelectObjective` (`KismetMathLibrary.Conv_IntToBool` _team) ControlledPawn))

(fn `EnemyHasTheFlag`
  (returns (EnemyHasTheFlag :type Boolean))
  (bind _flag (`self.GetFlag` (`self.Team`)))
  (return (`/Game/FPS/Blueprints/GameObjectives/CTF_Flag/BP_BaseFlag.bFlagTaken` _flag)))

(fn `GetFlag`
  (params (bTeam :type Boolean))
  (returns (Flag :type "/Game/FPS/Blueprints/GameObjectives/CTF_Flag/BP_BaseFlag Object Reference"))
  (bind _gs (`self.GS`))
  (return (select `bool` bTeam :`false` (`/Game/FPS/Blueprints/GameModes/CaptureTheFlag/BP_CaptureTheFlag_GS.FlagTeam_0` _gs) :`true` (`/Game/FPS/Blueprints/GameModes/CaptureTheFlag/BP_CaptureTheFlag_GS.FlagTeam_1` _gs))))

(fn `SelectObjective`
  (params (Team :type Boolean) (ControlledPawn :type "Pawn Object Reference"))
  (set `self.Team` Team)
  (set `self.Controlled Pawn` ControlledPawn)
  (bind _asbp_capture_the_flag_gs (cast `/Game/FPS/Blueprints/GameModes/CaptureTheFlag/BP_CaptureTheFlag_GS` (`GameplayStatics.GetGameState`)))
  (set `self.GS` _asbp_capture_the_flag_gs)
  (bind _enemyhastheflag (`self.EnemyHasTheFlag`))
  (if _enemyhastheflag
    ;[1 1 1] 枪回旗子
    (bind _flag (`self.GetFlag` (not (`self.Team`))))
    (`BTFunctionLibrary.SetBlackboardValueAsVector` (`self.Vectorkey`) (`NavigationSystemV1.K2_GetRandomReachablePointInRadius` (`Actor.K2_GetActorLocation` _flag) 100.0 null null))
    (else
      (bind _bteamhastheflag (`self.TeamHasTheFlag`))
      (if _bteamhastheflag
        (bind _flag_2 (`self.GetFlag` (not (`self.Team`)))) ; 敌方旗帜
        (bind _carrier (`/Game/FPS/Blueprints/GameObjectives/CTF_Flag/BP_BaseFlag.Carrier` _flag_2))
        (if (== (`self.Controlled Pawn`) _carrier)
          ;[1 1 1] 将旗帜带到基地
          (bind _flag_3 (`self.GetFlag` (`self.Team`)))
          (`BTFunctionLibrary.SetBlackboardValueAsVector` (`self.Vectorkey`) (`/Game/FPS/Blueprints/GameObjectives/CTF_Flag/BP_BaseFlag.InitialPossition` _flag_3))
          (else
            ;[1 1 1] 保卫旗帜携带者
            (`BTFunctionLibrary.SetBlackboardValueAsVector` (`self.Vectorkey`) (`NavigationSystemV1.K2_GetRandomReachablePointInRadius` (`Actor.K2_GetActorLocation` _carrier) 1000.0 null null))))
        (else
          ;[1 1 1] 夺取敌人的旗帜
          (bind _flag_4 (`self.GetFlag` (not (`self.Team`))))
          (`BTFunctionLibrary.SetBlackboardValueAsVector` (`self.Vectorkey`) (`Actor.K2_GetActorLocation` _flag_4)))))))

(fn `TeamHasTheFlag`
  (returns (bTeamHasTheFlag :type Boolean))
  (bind _flag (`self.GetFlag` (not (`self.Team`))))
  (return (`/Game/FPS/Blueprints/GameObjectives/CTF_Flag/BP_BaseFlag.bFlagTaken` _flag)))