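; Behavior tree task that picks a random reachable point near the Objective actor for an AI, such as around an interactable.
; It reads the Objective actor from the blackboard, queries the navigation system within a fixed radius of its location, and writes the result to the Location key.
; It only sets the key without moving the pawn, and finishes successfully even when no point is found or the task is aborted.
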(event `self.ReceiveExecuteAI`
  (params (OwnerController :type "AIController Object Reference") (ControlledPawn :type "Pawn Object Reference"))
  (bind _returnvalue (`BTFunctionLibrary.GetBlackboardValueAsActor` (`self.Objective`)))
  (bind (_randomlocation _returnvalue_2) (`NavigationSystemV1.K2_GetRandomReachablePointInRadius` (`Actor.K2_GetActorLocation` _returnvalue) 500.0 null null))
  ;[1 1 1] 交互物位置
  (`/Engine/EditorBlueprintResources/StandardMacros.IsValid` _returnvalue
    (:`Is Valid`
      (if _returnvalue_2
        (`BTFunctionLibrary.SetBlackboardValueAsVector` (`self.Location`) _randomlocation)))
    (:`Is Not Valid`
      _))
  (`self.FinishExecute` true))

(event `self.ReceiveAbortAI`
  (params (OwnerController :type "AIController Object Reference") (ControlledPawn :type "Pawn Object Reference"))
  (`self.FinishExecute` true))