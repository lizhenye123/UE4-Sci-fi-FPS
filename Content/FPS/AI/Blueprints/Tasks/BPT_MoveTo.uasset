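; Behavior tree task that makes an AI pawn run to the blackboard Objective actor or Location vector.
; It wraps AI MoveTo, setting the BP_BaseCharacter Running flag and raising max walk speed during the move, then restoring walking on finish or abort.
; Failed moves still finish as success, and abort calls FinishExecute rather than FinishAbort.
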(event `self.ReceiveExecuteAI`
  (params (OwnerController :type "AIController Object Reference") (ControlledPawn :type "Pawn Object Reference"))
  (`self.SetRunning` ControlledPawn true)
  (`|AIMoveTo` ControlledPawn (`BTFunctionLibrary.GetBlackboardValueAsVector` (`self.Location`)) (`BTFunctionLibrary.GetBlackboardValueAsActor` (`self.Objective`)) (`self.AcceptanceRadius`)
    (:`OnSuccess`
      _)
    (:`OnFail`
      _))
  (`self.SetRunning` ControlledPawn)
  (`self.FinishExecute` true))

(event `self.ReceiveAbortAI`
  (params (OwnerController :type "AIController Object Reference") (ControlledPawn :type "Pawn Object Reference"))
  (`self.SetRunning` ControlledPawn)
  (`self.FinishExecute` true))

(fn `SetRunning`
  (params (Pawn :type "Pawn Object Reference") (bRun :type Boolean))
  (bind _asbp_base_character (cast `/Game/FPS/Blueprints/CharacterAndClasses/BP_BaseCharacter` Pawn))
  (set `/Game/FPS/Blueprints/CharacterAndClasses/BP_BaseCharacter.bRunning` bRun _asbp_base_character)
  (set `CharacterMovementComponent.MaxWalkSpeed` (select `bool` bRun :`false` 400.0 :`true` 600.0 :!type "Float (single-precision)") (`Character.CharacterMovement` _asbp_base_character)))