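; Networked ammo box interactable that refills the ammunition of the character who uses it.
; Interact calls a server event that sends the instigator a refill message, multicasts a positional refill sound and forces a net update.
; The sound plays only where cosmetic events can execute.
; Interaction getters supply a description and short interact time, while the icon is empty and TryToInteract always returns false.
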(event `/Game/FPS/Blueprints/Interfaces/iInteractive.Interact`
  (params (Instigator :type "Character Object Reference"))
  ;[1 1 1] 为角色添加弹药
  (`self.Server_AddAmmo` Instigator))

(event `Server_AddAmmo`
  (params (Instigator :type "Actor Object Reference"))
  ;[1 1 1] 服务器添加弹药
  (message `/Game/FPS/Blueprints/Interfaces/iPawnActions.OnRefillAmmo` Instigator)
  (`self.Multicast_PlaySound`)
  (`self.ForceNetUpdate`))

(event `Multicast_PlaySound`
  ;[1 1 1] 广播补充弹药的声音
  (`/Engine/EditorBlueprintResources/StandardMacros.Can Execute Cosmetic Events`
    (:`True`
      (`GameplayStatics.PlaySoundAtLocation` (`self.RefillAmmoSound`) (`self.K2_GetActorLocation`) (struct) 0.8 1.0 0.0 "/Game/FPS/Sound/AudioSettings/Attenuation/ATT_Weapon.ATT_Weapon" null null))))

(fn `GetDescription`
  (returns (Description :type Text))
  (return "Refill ammunition"))

(fn `GetIcon`
  (returns (Icon :type "Texture Object Reference"))
  (return null))

(fn `GetInteractTime`
  (returns (InteractTime :type "Float (double-precision)"))
  (return 0.7))

(fn `TryToInteract`
  (returns (bFailure :type Boolean))
  (return false))

(fn `UserConstructionScript`)