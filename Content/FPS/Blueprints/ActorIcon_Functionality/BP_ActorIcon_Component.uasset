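; BP_ActorIcon_Component is a proximity icon, using its parent actor's instigator for team, that shows a widget message to the local player.
; BeginPlay creates the widget; on authority it checks existing overlaps and, if UseTeam is set, takes the instigator's team.
; Sphere overlaps show or hide the message for player pawn 0, optionally same-team only.
; Team's OnRep rechecks players inside, and the construction script sizes the sphere.
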(event `self.ReceiveBeginPlay`
  ;[1 1 1] 显示窗口小部件在开始播放
  (bind _returnvalue (`|CreateWidget` (`self.WidgetClass`)))
  (`WidgetComponent.SetWidget` (`self.Icon_Widget`) _returnvalue)
  (`/Engine/EditorBlueprintResources/ActorMacros.Switch Has Authority`
    (:`Authority`
      (`self.CheckPlayersInside`)
      (if (`self.bUseTeam`)
        (set `self.Team` (`/Game/FPS/Blueprints/FunctionLibrary/BP_FunctionLibrary.GetPlayerTeamFromPlayerState` (`Pawn.PlayerState` (`Actor.Instigator` (`self.GetParentActor`)))))))))

(event `CheckPlayersInside`
  (bind _returnvalue (`GameplayStatics.GetPlayerPawn` 0))
  ;[1 1 1] 显示窗口小部件在开始播放
  (for _array_element (`PrimitiveComponent.GetOverlappingActors` (`self.CollisionSphere`) "/Script/Engine.Character")
    (if (== _array_element _returnvalue)
      (if (or (== (`self.Team`) (`/Game/FPS/Blueprints/FunctionLibrary/BP_FunctionLibrary.GetPlayerTeamFromPlayerState` (`Pawn.PlayerState` _returnvalue))) (not (`self.bUseTeam`)))
        (message `/Game/FPS/Blueprints/Interfaces/iUI.ShowWidget` (`WidgetComponent.GetUserWidgetObject` (`self.Icon_Widget`)))))))

(event `self.CollisionSphere.OnComponentBeginOverlap`
  (params (OverlappedComponent :type "PrimitiveComponent Object Reference") (OtherActor :type "Actor Object Reference") (OtherComp :type "PrimitiveComponent Object Reference") (OtherBodyIndex :type Integer) (bFromSweep :type Boolean) (SweepResult :type "HitResult Structure (by ref)"))
  ;[1 1 1] 重叠的时候显示UI
  (if (== OtherActor (`GameplayStatics.GetPlayerPawn` 0))
    (bind _aspawn (cast `Pawn` OtherActor))
    (if (or (== (`/Game/FPS/Blueprints/FunctionLibrary/BP_FunctionLibrary.GetPlayerTeamFromPlayerState` (`Pawn.PlayerState` _aspawn)) (`self.Team`)) (not (`self.bUseTeam`)))
      (message `/Game/FPS/Blueprints/Interfaces/iUI.ShowWidget` (`WidgetComponent.GetUserWidgetObject` (`self.Icon_Widget`))))))

(event `self.CollisionSphere.OnComponentEndOverlap`
  (params (OverlappedComponent :type "PrimitiveComponent Object Reference") (OtherActor :type "Actor Object Reference") (OtherComp :type "PrimitiveComponent Object Reference") (OtherBodyIndex :type Integer))
  ;[1 1 1] 离开的时候隐藏UI
  (if (== OtherActor (`GameplayStatics.GetPlayerPawn` 0))
    (bind _aspawn (cast `Pawn` OtherActor))
    (if (or (== (`/Game/FPS/Blueprints/FunctionLibrary/BP_FunctionLibrary.GetPlayerTeamFromPlayerState` (`Pawn.PlayerState` _aspawn)) (`self.Team`)) (not (`self.bUseTeam`)))
      (message `/Game/FPS/Blueprints/Interfaces/iUI.HideWidget` (`WidgetComponent.GetUserWidgetObject` (`self.Icon_Widget`))))))

(fn `OnRep_Team`
  (`self.CheckPlayersInside`))

(fn `UserConstructionScript`
  (`SphereComponent.SetSphereRadius` (`self.CollisionSphere`) (`self.SetWidgetActionRadius`) true))