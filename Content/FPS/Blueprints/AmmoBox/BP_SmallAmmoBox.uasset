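; A thrown small ammo box pickup that resupplies the current weapon of a character needing ammo, then destroys itself.
; The server launches it with the instigator's velocity, arms it after a short delay, checks existing overlaps and limits its lifespan.
; A looping timer stops physics, and movement replication on the server, once the box rests.
; Server overlaps attempt pickup and award the instigator score for same-team pawns, even if no ammo is taken.
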(event `self.ReceiveBeginPlay`
  ;[1 1 1] 延迟开始播放时激活
  (`|ExecutionSequence`
    (:`then_0`
      (`/Engine/EditorBlueprintResources/ActorMacros.Switch Has Authority`
        (:`Authority`
          (`self.AddInitialImpulse`)
          (`KismetSystemLibrary.K2_SetTimerDelegate` (delegate `Init_Medkit`) 2.0)
          (`self.SetLifeSpan` 30.0))))
    (:`then_1`
      (bind _returnvalue (`KismetSystemLibrary.K2_SetTimerDelegate` (delegate `StopSimulatingPhysics`) 1.0 true))
      (set `self.CheckVelocityTimerHandle` _returnvalue))))

(event `Init_Medkit`
  ;[1 1 1] 延迟开始播放时激活
  (set `self.bActive` true)
  (`self.FindOverlappingActorOnActivation`))

(event `StopSimulatingPhysics`
  ;[1 1 1] 延迟开始播放时激活
  ;;[1 1 1] 如果速度为 0，则停止模拟物理
  (if (not (!= (`SceneComponent.GetComponentVelocity` (`self.StaticMesh`)) (0.0 0.0 0.0) :`ErrorTolerance` 0.01))
    (`PrimitiveComponent.SetSimulatePhysics` (`self.StaticMesh`) false)
    (`KismetSystemLibrary.K2_ClearAndInvalidateTimerHandle` (`self.CheckVelocityTimerHandle`))
    (`/Engine/EditorBlueprintResources/ActorMacros.Switch Has Authority`
      (:`Authority`
        (`self.SetReplicateMovement` false)))))

(event `self.InfluenceSphere.OnComponentBeginOverlap`
  (params (OverlappedComponent :type "PrimitiveComponent Object Reference") (OtherActor :type "Actor Object Reference") (OtherComp :type "PrimitiveComponent Object Reference") (OtherBodyIndex :type Integer) (bFromSweep :type Boolean) (SweepResult :type "HitResult Structure (by ref)"))
  (bind _instigator (`self.Instigator`))
  (bind _playerstate (`Pawn.PlayerState` _instigator))
  ;[1 1 1] 子弹让捡了后
  (`/Engine/EditorBlueprintResources/ActorMacros.Switch Has Authority`
    (:`Authority`
      (`self.Use` OtherActor)
      (bind _aspawn (cast `Pawn` OtherActor))
      (if (and (!= OtherActor _instigator) (== (`/Game/FPS/Blueprints/FunctionLibrary/BP_FunctionLibrary.GetPlayerTeamFromPlayerState` _playerstate) (`/Game/FPS/Blueprints/FunctionLibrary/BP_FunctionLibrary.GetPlayerTeamFromPlayerState` (`Pawn.PlayerState` _aspawn))))
        (message `/Game/FPS/Blueprints/Interfaces/iPlayerState.AddScoreToPlayer` _playerstate 30.0 "NewEnumerator5")))))

(fn `AddInitialImpulse`
  (`PrimitiveComponent.AddImpulse` (`self.StaticMesh`) (+ (* (`self.GetActorForwardVector`) 9000.0) (* (`MovementComponent.Velocity` (`Character.CharacterMovement` (cast `Character` (`self.Instigator`) :!pure true))) 20.0)) "None" false))

(fn `FindOverlappingActorOnActivation`
  (locals (OverlappingActor :type "Character Object Reference"))
  (bind _overlappingactor (`local.OverlappingActor`))
  (bind _influencesphere (`self.InfluenceSphere`))
  (`/Engine/EditorBlueprintResources/StandardMacros.IsValid` _influencesphere
    (:`Is Valid`
      (for _array_element (`PrimitiveComponent.GetOverlappingActors` _influencesphere "/Script/Engine.Character")
        (bind _ascharacter (cast `Character` _array_element))
        (bind _bneedsammo (message `/Game/FPS/Blueprints/Interfaces/iPawnActions.CharacterdNeedsAmmo` _ascharacter))
        (if _bneedsammo
          (set `local.OverlappingActor` _ascharacter)))
      ;[1 1 1] 如果 medkit 可用于某人将在激活时使用
      (`/Engine/EditorBlueprintResources/StandardMacros.IsValid` _overlappingactor
        (:`Is Valid`
          (`self.Use` _overlappingactor))))))

(fn `Use`
  (params (Actor :type "Actor Object Reference"))
  (if (`self.bActive`)
    (bind _ascharacter (cast `Character` Actor))
    (bind _bneedsammo (message `/Game/FPS/Blueprints/Interfaces/iPawnActions.CharacterdNeedsAmmo` _ascharacter))
    (if _bneedsammo
      (set `self.bActive` false)
      (message `/Game/FPS/Blueprints/Interfaces/iPawnActions.AddAmmoToCurrentWeapon` _ascharacter)
      (`ActorComponent.K2_DestroyComponent` (`self.WidgetActor`))
      (`self.K2_DestroyActor`)
      (return))))

(fn `UserConstructionScript`)