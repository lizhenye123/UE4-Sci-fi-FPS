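; Frag grenade lethal equipment that the player can cook before throwing.
; Activate starts a fuse timer and shows a cooking widget; release or drop passes the remaining time to a server-spawned BP_FragGrenade.
; Throws spawn ahead of the camera with upward-pitched control rotation, while drops and in-hand explosions spawn at the third-person mesh.
; A successful spawn triggers a client event that tells the owner to reduce lethal ammo.
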(event `Server_SpawnGrenade`
  (params (TimeLeft :type "Float (double-precision)") (`Spawn Transform Location` :type "Vector Structure"))
  (bind _returnvalue (`self.GetOwner`))
  (bind _returnvalue_2 (`self.GetInstigatorController` _returnvalue))
  (bind (_returnvalue_roll _returnvalue_pitch _returnvalue_yaw) (`KismetMathLibrary.BreakRotator` (`Controller.GetControlRotation` _returnvalue_2)))
  ;[1 1 1] Grenade
  ;;[1 1 1] 生成手榴弹
  (bind _returnvalue_3 (`|SpawnActorFromClass` "/Game/FPS/Blueprints/Grenade/BP_FragGrenade.BP_FragGrenade_C" (`KismetMathLibrary.MakeTransform` `Spawn Transform Location` (`KismetMathLibrary.MakeRotator` _returnvalue_roll (+ _returnvalue_pitch 15.0) _returnvalue_yaw)) "Undefined" "OverrideRootScale" _returnvalue_2 TimeLeft 0.0 (cast `Pawn` _returnvalue :!pure true)))
  (`/Engine/EditorBlueprintResources/StandardMacros.IsValid` _returnvalue_3
    (:`Is Valid`
      (`self.Client_ReduceLethalAmmo`))))

(event `self.ReleaseLethal`
  ;[1 1 1] Grenade
  ;;[1 1 1] 释放特殊武器
  (bind _asplayer_controller (cast `PlayerController` (`self.GetInstigatorController` (`self.GetOwner`))))
  (`self.Server_SpawnGrenade` (`KismetSystemLibrary.K2_GetTimerRemainingTimeHandle` (`self.CookGrenadeTimer`)) (`KismetMathLibrary.MakeVector` (.x (+ (`PlayerCameraManager.GetCameraLocation` (`PlayerController.PlayerCameraManager` _asplayer_controller)) (* (`self.GetActorForwardVector` _asplayer_controller) 100.0))) (.y (+ (`PlayerCameraManager.GetCameraLocation` (`PlayerController.PlayerCameraManager` _asplayer_controller)) (* (`self.GetActorForwardVector` _asplayer_controller) 100.0))) (+ (.z (+ (`PlayerCameraManager.GetCameraLocation` (`PlayerController.PlayerCameraManager` _asplayer_controller)) (* (`self.GetActorForwardVector` _asplayer_controller) 100.0))) 30.0))))

(event `self.OnRelease`
  ;[1 1 1] Grenade
  ;;[1 1 1] 释放
  (bind _cookinggrenadewidget (`self.CookingGrenadeWidget`)
    (:`then`
      (`Widget.RemoveFromParent` _cookinggrenadewidget)
      (set `self.bReleased` true)
      (`KismetSystemLibrary.K2_ClearAndInvalidateTimerHandle` (`self.CookGrenadeTimer`)))
    (:`else`)))

(event `Reset`
  ;[1 1 1] Grenade
  (set `self.bReleased` false)
  (`KismetSystemLibrary.K2_ClearAndInvalidateTimerHandle` (`self.CookGrenadeTimer`)))

(event `Client_ReduceLethalAmmo`
  ;[1 1 1] Grenade
  ;;[1 1 1] 减少手榴弹数量
  (message `/Game/FPS/Blueprints/Interfaces/iPawnActions.ReduceLethalAmmo` (`self.GetOwner`)))

(event `self.Activate`
  ;[1 1 1] Grenade
  ;;[1 1 1] 拉开手榴弹了，但是没放
  (`self.Reset`)
  (bind _returnvalue (`KismetSystemLibrary.K2_SetTimerDelegate` (delegate `ExplodeGrenade`) (`self.TimeToExplode`)))
  (set `self.CookGrenadeTimer` _returnvalue)
  (bind _returnvalue_2 (`|CreateWidget` "/Game/FPS/UI/Gameplay/WB_CookingGrenade.WB_CookingGrenade_C" (`GameplayStatics.GetPlayerController` 0)))
  (bind _output_get (set `self.CookingGrenadeWidget` _returnvalue_2))
  (`UserWidget.AddToViewport` _output_get 0))

(event `self.DropLethal`
  (bind _cookgrenadetimer (`self.CookGrenadeTimer`))
  ;[1 1 1] Grenade
  ;;[1 1 1] 掉落手榴弹
  (set `self.bReleased` true)
  (if (`KismetSystemLibrary.K2_IsTimerActiveHandle` _cookgrenadetimer)
    (`self.Server_SpawnGrenade` (`KismetSystemLibrary.K2_GetTimerRemainingTimeHandle` _cookgrenadetimer) (`SceneComponent.K2_GetComponentLocation` (`self.TPP_Mesh`)))
    (`KismetSystemLibrary.K2_ClearAndInvalidateTimerHandle` _cookgrenadetimer)))

(event `ExplodeGrenade`
  ;[1 1 1] Grenade
  ;;[1 1 1] 拉开手榴弹了，但是没放
  (if (not (`self.bReleased`))
    (`Widget.RemoveFromParent` (`self.CookingGrenadeWidget`))
    (`self.Server_SpawnGrenade` 0.01 (`SceneComponent.K2_GetComponentLocation` (`self.TPP_Mesh`)))))

(fn `UserConstructionScript`
  (`parent.UserConstructionScript`)
  (set `self.UI_Icon` "/Game/FPS/UI/Textures/T_FragGrenadeIcon.T_FragGrenadeIcon"))