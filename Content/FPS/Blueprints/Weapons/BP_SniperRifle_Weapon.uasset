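; Sniper rifle weapon Blueprint that adds a scope overlay and shot camera shake to a parent weapon class.
; Aiming creates the WB_SniperScope widget and hides the pawn's first- or third-person mesh through message calls.
; Stopping aim removes the scope, stops camera shakes and restores that mesh.
; Shots play FireShake when aimed, otherwise CS_FireWeapon, and WeaponVisibility toggles owner visibility of the first-person weapon mesh.
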(event `self.OnBeginAiming`
  (bind _returnvalue (`GameplayStatics.GetPlayerPawn` 0))
  ;[1 1 1] 开始瞄准
  (bind _returnvalue_2 (`|CreateWidget` "/Game/FPS/UI/Gameplay/WB_SniperScope.WB_SniperScope_C" (`GameplayStatics.GetPlayerController` 0)))
  (bind _output_get (set `self.SniperScopeRef` _returnvalue_2))
  (`UserWidget.AddToViewport` _output_get -1)
  (bind _busingtpp (message `/Game/FPS/Blueprints/Interfaces/iPawnActions.UsingTPP` _returnvalue))
  (if _busingtpp
    (message `/Game/FPS/Blueprints/Interfaces/iPawnActions.HideTPPMesh` _returnvalue)
    (else
      (message `/Game/FPS/Blueprints/Interfaces/iPawnActions.HideFPPMesh` _returnvalue))))

(event `self.OnStopAiming`
  (bind _returnvalue (`GameplayStatics.GetPlayerPawn` 0))
  ;[1 1 1] 结束瞄准
  (`PlayerCameraManager.StopAllCameraShakes` (`GameplayStatics.GetPlayerCameraManager` 0) true)
  (`Widget.RemoveFromParent` (`self.SniperScopeRef`))
  (bind _busingtpp (message `/Game/FPS/Blueprints/Interfaces/iPawnActions.UsingTPP` _returnvalue))
  (if _busingtpp
    (message `/Game/FPS/Blueprints/Interfaces/iPawnActions.ShowTPPMesh` _returnvalue)
    (else
      (message `/Game/FPS/Blueprints/Interfaces/iPawnActions.ShowFPPMesh` _returnvalue))))

(event `self.PlayShotShake`
  ;[1 1 1] 开火镜头晃动
  (bind _baiming (message `/Game/FPS/Blueprints/Interfaces/iPawnActions.IsAiming` (`GameplayStatics.GetPlayerPawn` 0)))
  (`PlayerCameraManager.StartCameraShake` :`self` (`GameplayStatics.GetPlayerCameraManager` 0) :`ShakeClass` (select `bool` _baiming :`false` "/Game/FPS/Blueprints/CameraShake/CS_FireWeapon.CS_FireWeapon_C" :`true` (`self.FireShake`))))

(fn `UserConstructionScript`
  (`parent.UserConstructionScript`))

(fn `WeaponVisibility`
  (params (bVisible :type Boolean))
  (`PrimitiveComponent.SetOwnerNoSee` (`self.MeshFPP`) (not bVisible)))