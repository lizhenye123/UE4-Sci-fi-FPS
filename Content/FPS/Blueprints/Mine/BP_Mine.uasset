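; BP_Mine is a mine that explodes when a Character overlaps its Sphere or when it takes damage.
; Overlap triggers only on authority, while a Destroyed flag keeps repeated damage from re-entering the blast.
; Both paths deal full radial damage from slightly above the mine, credited to ControllerInstigator, then destroy the actor after a short delay.
; A multicast plays explosion particles, sound and camera shake where cosmetic events can run.
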(event `self.Sphere.OnComponentBeginOverlap`
  (params (OverlappedComponent :type "PrimitiveComponent Object Reference") (OtherActor :type "Actor Object Reference") (OtherComp :type "PrimitiveComponent Object Reference") (OtherBodyIndex :type Integer) (bFromSweep :type Boolean) (SweepResult :type "HitResult Structure (by ref)"))
  ;[1 1 1] 开始重叠
  (`/Engine/EditorBlueprintResources/ActorMacros.Switch Has Authority`
    (:`Authority`
      (cast `Character` OtherActor)
      (`GameplayStatics.ApplyRadialDamage` 150.0 (`KismetMathLibrary.MakeVector` (.x (`self.K2_GetActorLocation` self)) (.y (`self.K2_GetActorLocation` self)) (+ (.z (`self.K2_GetActorLocation` self)) 30.0)) (`self.Radius`) "/Game/FPS/Blueprints/Weapons/DamageTypes/DT_Explosion.DT_Explosion_C" (`|MakeArray` self :!type "Actor Object Reference") null (`self.ControllerInstigator`) true :!label _label)
      (`self.Multicats_PlayEffects`)
      (`KismetSystemLibrary.Delay` 0.1)
      (`self.K2_DestroyActor`))))

(event `self.ReceiveAnyDamage`
  (params (Damage :type "Float (single-precision)") (DamageType :type "DamageType Object Reference") (InstigatedBy :type "Controller Object Reference") (DamageCauser :type "Actor Object Reference"))
  ;[1 1 1] 开始重叠
  (if (not (`self.bDestroyed`))
    (set `self.bDestroyed` true)
    (goto _label)))

(event `Multicats_PlayEffects`
  (bind _radius (`self.Radius`))
  (bind _returnvalue (`self.K2_GetActorLocation` self))
  ;[1 1 1] 播放特效
  (`/Engine/EditorBlueprintResources/StandardMacros.Can Execute Cosmetic Events`
    (:`True`
      (`GameplayStatics.SpawnEmitterAtLocation` "/Game/FPS/Effects/WeaponEffects/Explosion/P_Explosion.P_Explosion" _returnvalue (struct) (3.0 3.0 3.0))
      (`GameplayStatics.PlaySoundAtLocation` null _returnvalue (struct) 1.0 1.0 0.0 null null null)
      (`GameplayStatics.PlayWorldCameraShake` "/Game/FPS/Blueprints/CameraShake/CS_Explosion.CS_Explosion_C" (0.0 0.0 0.0) (* _radius 2.0) (* _radius 3.0)))))

(fn `UserConstructionScript`)