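; Blueprint Interface for FPS pawns, letting other objects drive and query a character's combat actions without casting to its class.
; Action messages cover firing, reloading, melee (including AI), throwables, ammo and weapon pickup, first/third-person mesh visibility, equip animations, hit markers and death.
; Queries report health, ammo and explosive needs, aiming, death, view mode and current weapon.
; It declares signatures only, leaving behavior to implementing classes.
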(fn `AddAmmo`
  (params (AmmoType :type "/Game/FPS/Blueprints/Enums/EAmmoType Enum" :default "NewEnumerator0")))

(fn `AddAmmoToCurrentWeapon`)

(fn `AddLethalAmmo`)

(fn `AIUseMelee`)

(fn `CharacterdNeedsAmmo`
  (returns (bNeedsAmmo :type Boolean))
  (return false))

(fn `CharacterNeedsExplosives`
  (returns (bNeedsExplosives :type Boolean))
  (return false))

(fn `DestroyPawnWeapon`)

(fn `FireWeapon`)

(fn `GetCurrentWeapon`
  (returns (CurrentWeapon :type "/Game/FPS/Blueprints/Weapons/BP_BaseWeapon Object Reference"))
  (return null))

(fn `HideFPPMesh`)

(fn `HideLethalEquipment`)

(fn `HideTPPMesh`)

(fn `HideWeapon`)

(fn `IsAiming`
  (returns (bAiming :type Boolean))
  (return false))

(fn `IsCharacterFullHP`
  (returns (bIsFullHp :type Boolean))
  (return false))

(fn `IsDead`
  (returns (bIsDead :type Boolean))
  (return false))

(fn `OnMeleeCompleted`)

(fn `OnPickupWeapon`
  (params (WeaponClass :type "/Game/FPS/Blueprints/Weapons/BP_BaseWeapon Class Reference") (CurrentAmmo :type Integer)))

(fn `OnPlayerKilled`)

(fn `OnRefillAmmo`)

(fn `OnReloadCompleted`)

(fn `OnSuicide`)

(fn `OnWeaponInteract`
  (params (NewWeapon :type "/Game/FPS/Blueprints/Weapons/BP_BaseWeapon Object Reference")))

(fn `PlayFPPEquipWeapon`)

(fn `PlayTPPEquipWeapon`)

(fn `ReduceLethalAmmo`)

(fn `ShowFPPMesh`)

(fn `ShowHitMarker`
  (params (bIsVehicle :type Boolean)))

(fn `ShowLethalEquipment`)

(fn `ShowTPPMesh`)

(fn `ShowVehicleHitMarker`)

(fn `SpawnExplosive`)

(fn `StopFiringWeapon`)

(fn `StopPawn`)

(fn `ThrowItem`)

(fn `UsingTPP`
  (returns (bUsingTPP :type Boolean))
  (return false))