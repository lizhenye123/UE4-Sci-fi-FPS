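; BP_SpawnProtectedZone is a team spawn protection volume that punishes players who linger in an enemy spawn.
; Box overlaps react only to player 0's pawn and compare its PlayerState team to SpawnTeam.
; An intruder's entry starts a timer and shows a warning widget fed its handle; exit clears both, while expiry sends the pawn a suicide message.
; The construction script sizes the box from BoxX and BoxY with fixed height.
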(event `self.Box.OnComponentBeginOverlap`
  (params (OverlappedComponent :type "PrimitiveComponent Object Reference") (OtherActor :type "Actor Object Reference") (OtherComp :type "PrimitiveComponent Object Reference") (OtherBodyIndex :type Integer) (bFromSweep :type Boolean) (SweepResult :type "HitResult Structure (by ref)"))
  ;[1 1 1] 进入敌方重生点
  (if (== OtherActor (`GameplayStatics.GetPlayerPawn` 0))
    (bind _asbp_player_state (cast `/Game/FPS/Blueprints/PlayerState/BP_PlayerState` (`Controller.PlayerState` (`self.GetInstigatorController` OtherActor))))
    (if (not (== (`/Game/FPS/Blueprints/PlayerState/BP_PlayerState.Team` _asbp_player_state) (`self.SpawnTeam`)))
      (`self.Warn` true))))

(event `self.Box.OnComponentEndOverlap`
  (params (OverlappedComponent :type "PrimitiveComponent Object Reference") (OtherActor :type "Actor Object Reference") (OtherComp :type "PrimitiveComponent Object Reference") (OtherBodyIndex :type Integer))
  ;[1 1 1] 进入敌方重生点
  (if (== OtherActor (`GameplayStatics.GetPlayerPawn` 0))
    (bind _asbp_player_state (cast `/Game/FPS/Blueprints/PlayerState/BP_PlayerState` (`Controller.PlayerState` (`self.GetInstigatorController` OtherActor))))
    (if (not (== (`/Game/FPS/Blueprints/PlayerState/BP_PlayerState.Team` _asbp_player_state) (`self.SpawnTeam`)))
      (`self.Warn` false))))

(event `Warn`
  (params (bShowWarning :type Boolean))
  (bind _protectedzonewidget (`self.ProtectedZoneWidget`))
  ;[1 1 1] 进入敌方重生点
  (if bShowWarning
    (bind _returnvalue (`KismetSystemLibrary.K2_SetTimerDelegate` (delegate `KillPlayerIntruder`) (`self.TimeToLeave`)))
    (bind _output_get (set `self.LeaveProtectedZoneHandle` _returnvalue))
    (bind _returnvalue_2 (`|CreateWidget` "/Game/FPS/UI/Gameplay/WB_ProtectedZoneWarning.WB_ProtectedZoneWarning_C" (`GameplayStatics.GetPlayerController` 0) _output_get))
    (`/Engine/EditorBlueprintResources/StandardMacros.IsValid` _returnvalue_2
      (:`Is Valid`
        (bind _output_get_2 (set `self.ProtectedZoneWidget` _returnvalue_2))
        (`UserWidget.AddToViewport` _output_get_2 0)))
    (else
      (`KismetSystemLibrary.K2_ClearAndInvalidateTimerHandle` (`self.LeaveProtectedZoneHandle`))
      (`/Engine/EditorBlueprintResources/StandardMacros.IsValid` _protectedzonewidget
        (:`Is Valid`
          (`Widget.RemoveFromParent` _protectedzonewidget))))))

(event `KillPlayerIntruder`
  ;[1 1 1] 进入敌方重生点
  (message `/Game/FPS/Blueprints/Interfaces/iPawnActions.OnSuicide` (`GameplayStatics.GetPlayerPawn` 0)))

(fn `UserConstructionScript`
  (`BoxComponent.SetBoxExtent` (`self.Box`) (`KismetMathLibrary.MakeVector` (`self.Box_X`) (`self.Box_Y`) 300.0) true))