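; Lobby game mode that runs map voting and launches the match on the winning map.
; It tracks joining and leaving players, opens each one's lobby menu, and pushes updated tallies for three maps to every controller after each vote.
; On launch it closes all lobby widgets, takes the first index with the highest count, and server-travels to Conquest, TeamDeathmatch or Rush, the default.
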(event `self.K2_PostLogin`
  (params (NewPlayer :type "PlayerController Object Reference"))
  ;[1 1 1] 玩家登录
  (`/Engine/EditorBlueprintResources/StandardMacros.IsValid` NewPlayer
    (:`Is Valid`
      (`KismetArrayLibrary.Array_Add` (`self.AllPlayerControllers`) NewPlayer)
      (bind _asbp_lobby_pc (cast `/Game/FPS/Blueprints/PlayerController/BP_LobbyPC` NewPlayer))
      (`/Game/FPS/Blueprints/PlayerController/BP_LobbyPC.Client_OpenLobbyMenu` _asbp_lobby_pc))))

(event `self.K2_OnLogout`
  (params (ExitingController :type "Controller Object Reference"))
  ;[1 1 1] 玩家退出
  (bind _asplayer_controller (cast `PlayerController` ExitingController))
  (`KismetArrayLibrary.Array_RemoveItem` (`self.AllPlayerControllers`) _asplayer_controller))

(event `LaunchGame`
  (bind _returnvalue (`GameplayStatics.GetPlayerController` 0))
  ;[1 1 1] 启动地图
  (`self.Server_CloseLobbyScreen`)
  (bind _maptolaunch (`self.SelectMapToPlay`))
  (switch `int` _maptolaunch
    (:`Default`
      (`KismetSystemLibrary.ExecuteConsoleCommand` "servertravel /Game/Maps/Levels/Rush" _returnvalue :!label _label))
    (:`0`
      (`KismetSystemLibrary.ExecuteConsoleCommand` "servertravel /Game/FPS/Maps/Conquest" _returnvalue))
    (:`1`
      (`KismetSystemLibrary.ExecuteConsoleCommand` "servertravel /Game/FPS/Maps/TeamDeathmatch" _returnvalue))
    (:`2`
      (goto _label))))

(event `Server_CloseLobbyScreen`
  ;[1 1 1] 关闭所有玩家的大厅UI
  (for _array_element (`self.AllPlayerControllers`)
    (bind _asbp_lobby_pc (cast `/Game/FPS/Blueprints/PlayerController/BP_LobbyPC` _array_element))
    (`/Game/FPS/Blueprints/PlayerController/BP_LobbyPC.Client_RemoveWidget` _asbp_lobby_pc)))

(event `Server_UpdateVotesForEveryone`
  ;[1 1 1] 为每个人设置地图投票
  (for _array_element (`self.AllPlayerControllers`)
    (bind _asbp_lobby_pc (cast `/Game/FPS/Blueprints/PlayerController/BP_LobbyPC` _array_element))
    (set `/Game/FPS/Blueprints/PlayerController/BP_LobbyPC.Map1Votes` (`self.Map1Votes`) _asbp_lobby_pc)
    (set `/Game/FPS/Blueprints/PlayerController/BP_LobbyPC.Map2Votes` (`self.Map2Votes`) _asbp_lobby_pc)
    (set `/Game/FPS/Blueprints/PlayerController/BP_LobbyPC.Map3Votes` (`self.Map3Votes`) _asbp_lobby_pc)))

(event `Server_IncreaseMapVotes`
  (params (Position :type Integer))
  ;[1 1 1] 增加地图票数
  (switch `int` Position
    (:`0`
      (set `self.Map1Votes` (+ (`self.Map1Votes`) 1)))
    (:`1`
      (set `self.Map2Votes` (+ (`self.Map2Votes`) 1)))
    (:`2`
      (set `self.Map3Votes` (+ (`self.Map3Votes`) 1))))
  (`self.Server_UpdateVotesForEveryone`))

(fn `SelectMapToPlay`
  (returns (MapToLaunch :type Integer))
  (locals (MapMoreVoted :type Byte))
  (bind _array (`|MakeArray` (`self.Map1Votes`) (`self.Map2Votes`) (`self.Map3Votes`)))
  (`KismetArrayLibrary.Array_Shuffle` _array)
  (for _array_element _array
    (if (> _array_element (`local.MapMoreVoted`))
      (set `local.MapMoreVoted` _array_element)))
  (for (_array_element_2 _array_index) _array
    (if (== _array_element_2 (`local.MapMoreVoted`))
      (return _array_index))))

(fn `UserConstructionScript`)