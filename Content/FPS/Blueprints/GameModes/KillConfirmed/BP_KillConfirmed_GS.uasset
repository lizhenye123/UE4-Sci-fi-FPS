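; Game State for the Kill Confirmed mode that tracks the dog tags dropped by dead players.
; On player death it projects the body's location onto the navmesh, spawns a BP_DogTag slightly above that point, sets its team and stores it in the Dogtags array.
; Removal takes a tag out of the array and destroys it.
; Team changes call the parent handler, then refresh every tag's material, which a separate event can also trigger.
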(event `UpdateDogtagsMaterial`
  (bind _dogtags (`self.Dogtags`))
  ;[1 1 1] 更新狗牌材质
  (if (`KismetArrayLibrary.Array_IsValidIndex` _dogtags)
    (for _array_element _dogtags
      (`/Engine/EditorBlueprintResources/StandardMacros.IsValid` _array_element
        (:`Is Valid`
          (`/Game/FPS/Blueprints/GameObjectives/KillConfirmDogTag/BP_DogTag.UpdateMaterial` _array_element))))))

(event `AddNewDogtag`
  (params (NewDogtag :type "/Game/FPS/Blueprints/GameObjectives/KillConfirmDogTag/BP_DogTag Object Reference"))
  ;[1 1 1] 添加狗牌
  (`KismetArrayLibrary.Array_AddUnique` (`self.Dogtags`) NewDogtag))

(event `RemoveDogTag`
  (params (DogtagToDelete :type "/Game/FPS/Blueprints/GameObjectives/KillConfirmDogTag/BP_DogTag Object Reference"))
  ;[1 1 1] 删除狗牌
  (`KismetArrayLibrary.Array_RemoveItem` (`self.Dogtags`) DogtagToDelete)
  (`self.K2_DestroyActor` DogtagToDelete))

(event `self.HandlePlayerDeath`
  (params (Team :type Integer) (DeadActor :type "Actor Object Reference") (Instigator :type "Controller Object Reference"))
  ;[1 1 1] 处理玩家死亡
  (bind _returnvalue (`|SpawnActorFromClass` "/Game/FPS/Blueprints/GameObjectives/KillConfirmDogTag/BP_DogTag.BP_DogTag_C" (`KismetMathLibrary.Conv_VectorToTransform` (`KismetMathLibrary.MakeVector` (.x (`NavigationSystemV1.K2_ProjectPointToNavigation` (`self.K2_GetActorLocation` DeadActor) null null (1000.0 1000.0 1000.0))) (.y (`NavigationSystemV1.K2_ProjectPointToNavigation` (`self.K2_GetActorLocation` DeadActor) null null (1000.0 1000.0 1000.0))) (+ (.z (`NavigationSystemV1.K2_ProjectPointToNavigation` (`self.K2_GetActorLocation` DeadActor) null null (1000.0 1000.0 1000.0))) 60.0))) "Undefined" "OverrideRootScale" DeadActor null))
  (`/Game/FPS/Blueprints/GameObjectives/KillConfirmDogTag/BP_DogTag.SetTeam` _returnvalue Team)
  (`self.AddNewDogtag` _returnvalue))

(event `self.HandlePlayerChangeTeam`
  ;[1 1 1] 更新材料 瞄准到的人的标签
  (`parent.HandlePlayerChangeTeam`)
  (for _array_element (`self.Dogtags`)
    (`/Game/FPS/Blueprints/GameObjectives/KillConfirmDogTag/BP_DogTag.UpdateMaterial` _array_element)))

(fn `UserConstructionScript`)