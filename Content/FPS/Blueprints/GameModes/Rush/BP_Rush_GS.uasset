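; Game state for the Rush mode, running staged bomb objectives with a round timer and a replicated reinforcement pool.
; When a stage's bombs all reach their final state, it resets timer and reinforcements, activates new spawns and initializes the next bombs.
; Deaths outside team 0 drain reinforcements.
; Empty reinforcements or timeout ends the match unless a current-stage bomb's state blocks it, as does clearing the final stage.
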(event `StartMatchTimer`
  ;[1 1 1] 启动匹配计时器
  (bind _returnvalue (`KismetSystemLibrary.K2_SetTimerDelegate` (delegate `TimeOut`) (`self.RoundTime`)))
  (set `self.TimeLimitHandler` _returnvalue)
  (`KismetSystemLibrary.K2_SetTimerDelegate` (delegate `UpdateTime`) 1.0 true))

(event `UpdateTime`
  ;[1 1 1] 启动匹配计时器
  (`self.UpdateTimeLeft`))

(event `TimeOut`
  ;[1 1 1] 启动匹配计时器
  (bind _asbp_base_gm (cast `/Game/FPS/Blueprints/GameModes/BP_Base_GM` (`GameplayStatics.GetGameMode`)))
  (if (not (`/Game/FPS/Blueprints/GameModes/BP_Base_GM.IsGameOver` _asbp_base_gm))
    (set `self.bTimeOut` true)
    (`self.CheckWinCondition`)))

(event `ReduceReinforcements`
  ;[1 1 1] 减少再形成，并检查游戏是否已经结束
  (bind _result (`/Engine/EditorBlueprintResources/StandardMacros.DecrementInt` (`self.Reinforcements`))
    (:`  `
      (bind _output_get (set `self.Reinforcements` (`KismetMathLibrary.Clamp` _result 0 (`self.MaxReinforcements`))))
      (if (== _output_get 0)
        (`self.CheckWinCondition`)))))

(event `SetBombState`
  (params (NewState :type "/Game/FPS/Blueprints/Enums/EBombStateEnum Enum" :default "NewEnumerator0"))
  ;[1 1 1] 改变炸弹状态
  (set `self.BombState` NewState))

(event `CheckGameState`
  ;[1 1 1] 检查是否所有的炸弹都已被销毁
  (set `self.bChangeState` true)
  (for _array_element (`self.BombRef`)
    (`/Engine/EditorBlueprintResources/StandardMacros.IsValid` _array_element
      (:`Is Valid`
        (if (and (== (`self.State`) (`/Game/FPS/Blueprints/GameObjectives/RushObjective/BP_RushObjective.State` _array_element)) (`|EnumInequality` (`/Game/FPS/Blueprints/GameObjectives/RushObjective/BP_RushObjective.BombState` _array_element) "NewEnumerator3"))
          (set `self.bChangeState` false)))))
  (if (`self.bChangeState`)
    (`self.ChangeState`)
    (else
      (`self.CheckWinCondition`))))

(event `ChangeState`
  ;[1 1 1] 改变状态
  (if (== (`self.State`) (`self.FinalState`))
    (bind _asbp_base_gm (cast `/Game/FPS/Blueprints/GameModes/BP_Base_GM` (`GameplayStatics.GetGameMode`)))
    (`/Game/FPS/Blueprints/GameModes/BP_Base_GM.Server_EndGame` _asbp_base_gm)
    (else
      (`self.ResetTimer`)
      (bind _output_get (set `self.State` (+ (`self.State`) 1)))
      (bind _asbp_rush_gm (cast `/Game/FPS/Blueprints/GameModes/Rush/BP_Rush_GM` (`GameplayStatics.GetGameMode`)))
      (`/Game/FPS/Blueprints/GameModes/Rush/BP_Rush_GM.ActivateNewSpawns` _asbp_rush_gm _output_get)
      (`self.ResetReinforcements`)
      (`KismetSystemLibrary.Delay` 5.0)
      (for _array_element (`self.BombRef`)
        (`/Engine/EditorBlueprintResources/StandardMacros.IsValid` _array_element
          (:`Is Valid`
            (if (== (`/Game/FPS/Blueprints/GameObjectives/RushObjective/BP_RushObjective.State` _array_element) (`self.State`))
              (`/Game/FPS/Blueprints/GameObjectives/RushObjective/BP_RushObjective.InitBomb` _array_element))))))))

(event `StartGame`
  ;[1 1 1] 初始化目标/和炸弹
  (for _array_element (`self.BombRef`) :!label _label
    (if (== (`/Game/FPS/Blueprints/GameObjectives/RushObjective/BP_RushObjective.State` _array_element) (`self.State`))
      (`/Game/FPS/Blueprints/GameObjectives/RushObjective/BP_RushObjective.InitBomb` _array_element))))

(event `self.OnStartMatch`
  ;[1 1 1] 初始化目标/和炸弹
  (`KismetSystemLibrary.K2_SetTimerDelegate` (delegate `UpdateTimeLeftToSpawn`) 1.0 true)
  (`self.StartMatchTimer`)
  (goto _label))

(event `UpdateTimeLeftToSpawn`
  ;[1 1 1] 初始化目标/和炸弹
  (set `self.TimeLeftForNextSpawn` (`KismetSystemLibrary.K2_GetTimerRemainingTimeHandle` (`self.TimeToSpawnHandler`))))

(event `self.HandlePlayerDeath`
  (params (Team :type Integer) (DeadActor :type "Actor Object Reference") (Instigator :type "Controller Object Reference"))
  ;[1 1 1] 处理玩家的死亡
  (if (!= Team 0)
    (`self.ReduceReinforcements`)))

(event `self.HandlePlayerChangeTeam`
  ;[1 1 1] 关于球员更换团队
  (`parent.HandlePlayerChangeTeam`)
  (for _array_element (`self.BombRef`)
    (`/Game/FPS/Blueprints/GameObjectives/RushObjective/BP_RushObjective.UpdateWidget` _array_element)))

(event `ResetReinforcements`
  ;[1 1 1] 重置增援部队
  (set `self.Reinforcements` (`self.MaxReinforcements`))
  (`self.ForceNetUpdate`))

(event `ResetTimer`
  ;[1 1 1] 重置定时器
  (set `self.bTimeOut` false)
  (`KismetSystemLibrary.K2_ClearAndInvalidateTimerHandle` (`self.TimeLimitHandler`))
  (`self.StartMatchTimer`))

(event `CheckWinCondition`
  ;[1 1 1] 检查游戏结束条件
  (set `self.bEnd` true)
  (for _array_element (`self.BombRef`)
    (`/Engine/EditorBlueprintResources/StandardMacros.IsValid` _array_element
      (:`Is Valid`
        (if (and (`|EnumEquality` (`/Game/FPS/Blueprints/GameObjectives/RushObjective/BP_RushObjective.BombState` _array_element) "NewEnumerator1") (== (`/Game/FPS/Blueprints/GameObjectives/RushObjective/BP_RushObjective.State` _array_element) (`self.State`)))
          (set `self.bEnd` false)))))
  (if (and (== (`self.Reinforcements`) 0) (`self.bEnd`))
    (bind _asbp_base_gm (cast `/Game/FPS/Blueprints/GameModes/BP_Base_GM` (`GameplayStatics.GetGameMode`) :!label _label_2))
    (`/Game/FPS/Blueprints/GameModes/BP_Base_GM.Server_EndGame` _asbp_base_gm)
    (elif (and (`self.bEnd`) (`self.bTimeOut`))
      (goto _label_2))))

(fn `OnRep_Reinforcements`
  (`self.RushUpdateReinforcements`))

(fn `UserConstructionScript`
  (set `self.Reinforcements` (`self.MaxReinforcements`)))