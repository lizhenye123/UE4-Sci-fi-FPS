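; Free-for-all deathmatch game mode that gives each joining player and created bot a unique, incrementing team number.
; Player controllers and their kill points live in parallel arrays, updated on scoring and logout.
; Players spawn as their chosen class at random points from PlayerSpawnsA; bots use a team-filtered subset, and each used point is flagged unavailable.
; Until game over, bot controllers queued in the GameState possess fresh pawns and restart their behavior tree.
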(event `self.ReceiveBeginPlay`
  ;[1 1 1] Begin Play
  (`parent.ReceiveBeginPlay`))

(event `self.HandleStartingNewPlayer`
  (params (NewPlayer :type "PlayerController Object Reference"))
  (bind _returnvalue (+ (`self.TeamToAssign`) 1))
  ;[1 1 1] 处理启动新玩家
  (message `/Game/FPS/Blueprints/Interfaces/iPlayerState.SetTeam` (`Controller.PlayerState` NewPlayer) _returnvalue)
  (set `self.TeamToAssign` _returnvalue)
  (`/Engine/EditorBlueprintResources/ActorMacros.Switch Has Authority`
    (:`Authority`
      (`/Engine/EditorBlueprintResources/StandardMacros.IsValid` NewPlayer
        (:`Is Valid`
          (`KismetArrayLibrary.Array_Add` (`self.AllPlayersPCs`) NewPlayer)
          (`KismetArrayLibrary.Array_AddUnique` (`self.AllPlayerPoints`) (make `/Game/FPS/Blueprints/GameModes/Deathmatch/PlayerPoints` (`Controller.PlayerState` NewPlayer))))))))

(event `Server_AddPoints`
  (params (PC :type "PlayerController Object Reference"))
  ;[1 1 1] 给玩家添加击杀数
  (for (_array_element _array_index) (`self.AllPlayersPCs`)
    (if (== _array_element PC)
      (bind (_output_playerstate _output_points) (break `/Game/FPS/Blueprints/GameModes/Deathmatch/PlayerPoints` (`|GetArrayItem` (`self.AllPlayerPoints`) _array_index)))
      (`KismetArrayLibrary.Array_Set` (`self.AllPlayerPoints`) _array_index (make `/Game/FPS/Blueprints/GameModes/Deathmatch/PlayerPoints` null (+ _output_points 1))))))

(event `self.K2_OnLogout`
  (params (ExitingController :type "Controller Object Reference"))
  ;[1 1 1] 玩家退出
  (bind _asbp_base_player_controller (cast `/Game/FPS/Blueprints/PlayerController/BP_BasePlayerController` ExitingController))
  (for (_array_element _array_index) (`self.AllPlayersPCs`)
    (if (== _asbp_base_player_controller _array_element)
      (`KismetArrayLibrary.Array_Remove` (`self.AllPlayerPoints`) _array_index)
      (`KismetArrayLibrary.Array_RemoveItem` (`self.AllPlayersPCs`) _array_element))))

(event `self.SpawnPlayerClass`
  (params (PlayerClass :type "/Game/FPS/Blueprints/Enums/EPlayerClass Enum" :default "NewEnumerator0") (PlayerController :type "PlayerController Object Reference"))
  (bind _playerspawnsa (`self.PlayerSpawnsA`))
  ;[1 1 1] 生成玩家类
  (if (`KismetArrayLibrary.Array_IsValidIndex` _playerspawnsa)
    (bind _output_get (set `self.SelectedSpawn` (`|GetArrayItem` _playerspawnsa (`KismetMathLibrary.RandomIntegerInRange` 0 (`KismetArrayLibrary.Array_LastIndex` _playerspawnsa)))))
    (set `/Game/FPS/Blueprints/PlayerSpawn/BP_PlayerSpawn.bCanBeUsed` false _output_get)
    (bind _returnvalue (`SceneComponent.K2_GetComponentToWorld` (`Actor.RootComponent` _output_get)))
    (bind _returnvalue_2 (`|SpawnActorFromClass` (select `/Game/FPS/Blueprints/Enums/EPlayerClass` PlayerClass :`NewEnumerator0` "/Game/FPS/Blueprints/CharacterAndClasses/BP_AssaultClass_A.BP_AssaultClass_A_C" :`NewEnumerator1` "/Game/FPS/Blueprints/CharacterAndClasses/BP_MedicClass_A.BP_MedicClass_A_C" :`NewEnumerator2` "/Game/FPS/Blueprints/CharacterAndClasses/BP_SupportClass_A.BP_SupportClass_A_C" :!type "Actor Class Reference") _returnvalue "Undefined" "OverrideRootScale" PlayerController null))
    (bind _aspawn (cast `Pawn` _returnvalue_2))
    (`Controller.Possess` PlayerController _aspawn)
    (bind _rotation (.rotation _returnvalue))
    (`Controller.SetControlRotation` PlayerController _rotation)
    (bind _asbp_base_player_controller (cast `/Game/FPS/Blueprints/PlayerController/BP_BasePlayerController` PlayerController))
    (`/Game/FPS/Blueprints/PlayerController/BP_BasePlayerController.Client_SetControlRotation` _asbp_base_player_controller _rotation)))

(event `self.CreateBots`
  (bind _teamabots (`self.TeamABots`))
  (bind _returnvalue (+ (`self.TeamToAssign`) 1))
  ;[1 1 1] 创建和生成机器人
  (if (> _teamabots 0)
    (for _ (range 1 (+ _teamabots 1))
      (bind _posiblespawn (`self.TeamPosibleSpawn` 0 (`self.PlayerSpawnsA`)))
      (if (`KismetArrayLibrary.Array_IsValidIndex` _posiblespawn)
        (bind _output_get (set `self.SelectedSpawn` (`|GetArrayItem` _posiblespawn (`KismetMathLibrary.RandomIntegerInRange` 0 (`KismetArrayLibrary.Array_LastIndex` _posiblespawn)))))
        (set `/Game/FPS/Blueprints/PlayerSpawn/BP_PlayerSpawn.bCanBeUsed` false _output_get)
        (bind (_returnvalue_location _returnvalue_rotation) (`KismetMathLibrary.BreakTransform` (`self.GetTransform` _output_get)))
        (bind _returnvalue_2 (`AIBlueprintHelperLibrary.SpawnAIFromClass` "/Game/FPS/Blueprints/AI_Characters/PlayerAI/BP_AI_Character_A.BP_AI_Character_A_C" (`self.AI_BehaviorTree`) _returnvalue_location _returnvalue_rotation true null))
        (`KismetArrayLibrary.Array_AddUnique` (`self.TeamABotsControllers`) (`Pawn.GetController` _returnvalue_2))
        (message `/Game/FPS/Blueprints/Interfaces/iPlayerState.SetTeam` (`Pawn.PlayerState` _returnvalue_2) _returnvalue)
        (set `self.TeamToAssign` _returnvalue)))))

(event `self.SpawnBots`
  ;[1 1 1] 创建和生成机器人
  (if (not (`self.IsGameOver`))
    (bind _asbp_base_gs (cast `/Game/FPS/Blueprints/GameModes/BP_Base_GS` (`GameplayStatics.GetGameState`)))
    (bind _botsreadytospawn (`/Game/FPS/Blueprints/GameModes/BP_Base_GS.BotsReadyToSpawn` _asbp_base_gs))
    (if (`KismetArrayLibrary.Array_IsValidIndex` _botsreadytospawn)
      (for _array_element _botsreadytospawn
        (bind _asbp_player_state (cast `/Game/FPS/Blueprints/PlayerState/BP_PlayerState` (`Controller.PlayerState` _array_element)))
        (bind _posiblespawn (`self.TeamPosibleSpawn` (`/Game/FPS/Blueprints/PlayerState/BP_PlayerState.Team` _asbp_player_state) (`self.PlayerSpawnsA`)))
        (if (`KismetArrayLibrary.Array_IsValidIndex` _posiblespawn)
          (bind _output_get (set `self.SelectedSpawn` (`|GetArrayItem` _posiblespawn (`KismetMathLibrary.RandomIntegerInRange` 0 (`KismetArrayLibrary.Array_LastIndex` _posiblespawn)))))
          (set `/Game/FPS/Blueprints/PlayerSpawn/BP_PlayerSpawn.bCanBeUsed` false _output_get)
          (bind (_returnvalue_location _returnvalue_rotation) (`KismetMathLibrary.BreakTransform` (`self.GetTransform` _output_get)))
          (bind _returnvalue (`|SpawnActorFromClass` "/Game/FPS/Blueprints/AI_Characters/PlayerAI/BP_AI_Character_A.BP_AI_Character_A_C" (`KismetMathLibrary.MakeTransform` _returnvalue_location _returnvalue_rotation) "AdjustIfPossibleButAlwaysSpawn" "OverrideRootScale" null null))
          (`/Engine/EditorBlueprintResources/StandardMacros.IsValid` _returnvalue
            (:`Is Valid`
              (`Controller.Possess` _array_element _returnvalue)
              (`AIController.RunBehaviorTree` (`AIBlueprintHelperLibrary.GetAIController` _returnvalue) (`self.AI_BehaviorTree`))))))
      (`KismetArrayLibrary.Array_Clear` _botsreadytospawn))))

(fn `UserConstructionScript`
  (`parent.UserConstructionScript`))