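; Blueprint function library of shared lookup helpers for the FPS game, covering ammo, player identity and match state.
; Magazine lookup returns the first entry matching an ammo type.
; Team and name getters forward message calls to the supplied object.
; Match queries cast the Game State to BP_Base_GS, with a default enum fallback for game mode but none for the game-over check.
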(fn `GetCurrentGameMode`
  (returns (CurrentGameMode :type "/Game/FPS/Blueprints/Enums/EGameModeNames Enum"))
  (bind _asbp_base_gs (cast `/Game/FPS/Blueprints/GameModes/BP_Base_GS` (`GameplayStatics.GetGameState` null))
    (:`then`
      (return (`/Game/FPS/Blueprints/GameModes/BP_Base_GS.CurrentGameMode` _asbp_base_gs)))
    (:`CastFailed`
      (return "NewEnumerator4"))))

(fn `GetMagazineInfoPerType`
  (params (Magazine :type "Array of /Game/FPS/Blueprints/CharacterAndClasses/AmmoMagazines Structure") (AmmoType :type "/Game/FPS/Blueprints/Enums/EAmmoType Enum" :default "NewEnumerator0"))
  (returns (`Array Element` :type "/Game/FPS/Blueprints/CharacterAndClasses/AmmoMagazines Structure"))
  (for _array_element Magazine
    (if (`|EnumEquality` (`.AmmoType_5_1CD642D04C3BF1F857D9EBBF2F2EF4F5` (break `/Game/FPS/Blueprints/CharacterAndClasses/AmmoMagazines` _array_element)) AmmoType)
      (return _array_element))))

(fn `GetPlayerNameFromPlayerState`
  (params (Object :type "PlayerState Object Reference"))
  (returns (PlayerName :type Text))
  (bind _playername (message `/Game/FPS/Blueprints/Interfaces/iPlayerState.GetName` Object))
  (return _playername))

(fn `GetPlayerTeamFromPlayerState`
  (params (Object :type "PlayerState Object Reference"))
  (returns (Team :type Integer))
  (bind _team (message `/Game/FPS/Blueprints/Interfaces/iPlayerState.GetTeam` Object))
  (return _team))

(fn `IsGameOver`
  (returns (bGameOver :type Boolean))
  (return (`/Game/FPS/Blueprints/GameModes/BP_Base_GS.IsGameOver` (cast `/Game/FPS/Blueprints/GameModes/BP_Base_GS` (`GameplayStatics.GetGameState` null) :!pure true))))