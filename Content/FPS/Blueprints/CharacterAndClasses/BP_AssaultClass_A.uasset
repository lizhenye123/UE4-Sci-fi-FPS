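; Assault class character for the FPS game, whose throwable item is a small ammo box.
; ThrowItem reuses the ServerSpawnMedKit call, passing the ammo box class instead of a med kit.
; Equipping plays the weapon's first-person montage, shows the weapon after a short timer to avoid a misplaced frame, and clears PerformingAction on completion.
; Unequipping plays its montage at double speed and hides the weapon on blend out.
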(event `/Game/FPS/Blueprints/Interfaces/iPawnActions.ThrowItem`
  ;[1 1 1] 设置子弹包
  (`self.Server_SpawnMedKit` "/Game/FPS/Blueprints/AmmoBox/BP_SmallAmmoBox.BP_SmallAmmoBox_C"))

(fn `UserConstructionScript`
  (`parent.UserConstructionScript`))