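; Support class character Blueprint whose throw-item ability has the server spawn a small explosive ammo box, reusing the med-kit spawn call.
; It plays the current weapon's first-person montages for equip and double-speed unequip.
; Equip briefly delays showing the weapon to avoid a one-frame wrong position and clears the performing-action flag on completion.
; Unequip hides the weapon as the montage blends out.
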(event `/Game/FPS/Blueprints/Interfaces/iPawnActions.ThrowItem`
  ;[1 1 1] 特殊弹药箱
  (`self.Server_SpawnMedKit` "/Game/FPS/Blueprints/AmmoBox/BP_SmallExplosiveAmmoBox.BP_SmallExplosiveAmmoBox_C"))

(fn `UserConstructionScript`
  (`parent.UserConstructionScript`))